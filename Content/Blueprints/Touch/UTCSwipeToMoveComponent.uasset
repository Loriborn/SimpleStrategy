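; Touch component for swipe-to-move input that turns single-finger drags into movement deltas.
; On touch it measures the change from the previous location scaled by Speed, then fires X, Y and location delta events alongside press and release events.
; With interpolation enabled, it stores a target delta and eases toward it on Tick via VInterpTo before broadcasting.
; Optional debug drawing shows a widget with the touch bounds while pressed.
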(event EventOnEventTouchMoved
  (params (Location :type Vector :default "0, 0, 0") (FingerIndex :type ETouchIndex%20Enum :default "Touch1"))
  (bind (_target_delta _current_delta) (CallFunction|RecalculateDelta Location))
  (bind _enable_interpolation (Variables|Configuration|GetEnable%20Interpolation))
  (bind _debug_widget (Variables|Temp|GetDebug%20Widget))
  (bind _returnvalue (not _enable_interpolation))
  (bind _returnvalue_2 (Math|Vector|SelectVector _target_delta _current_delta _returnvalue))
  (bind (_x _y) (Math|Vector|BreakVector _returnvalue_2))
  (|CallParentFunction Location FingerIndex)
  (if _returnvalue
    ;[0 0.25 1] Call Events
    (Default|CallOnDeltaXChanged _x)
    (Default|CallOnDeltaYChanged _y)
    (Default|CallOnDeltaLocationChanged _returnvalue_2)
    (else
      (Variables|Temp|SetTarget%20Delta _target_delta)
      (Variables|Temp|SetCurrent%20Delta _current_delta)))
  (Variables|Temp|SetPrevious%20Location Location)
  ;[1 0.25 0] Debug Drawing with Special Debug Widget
  (if (Variables|Default|GetEnable%20Debug%20Drawing)
    (Variables|/Game/Blueprints/Touch/UTCDebugWidget.UTCDebugWidget_C|SetBounds%20Origin _debug_widget (Variables|Default|GetBounds%20Origin))
    (Variables|/Game/Blueprints/Touch/UTCDebugWidget.UTCDebugWidget_C|SetBound%20Size _debug_widget (Variables|Default|GetBounds%20Size))))

(event EventOnEventTouchReleased
  (params (Location :type Vector :default "0, 0, 0") (FingerIndex :type ETouchIndex%20Enum :default "Touch1"))
  (bind (_target_delta _current_delta) (CallFunction|RecalculateDelta Location))
  (bind _debug_widget (Variables|Temp|GetDebug%20Widget))
  (|CallParentFunction Location FingerIndex)
  (if (not (Variables|Configuration|GetEnable%20Interpolation))
    _
    (else
      (Variables|Temp|SetTarget%20Delta _target_delta)
      (Variables|Temp|SetCurrent%20Delta _current_delta)))
  ;[0 0.25 1] Call Events
  (Default|CallOnReleased Location)
  ;[1 0.25 0] Debug Drawing with Special Debug Widget
  (if (Variables|Default|GetEnable%20Debug%20Drawing)
    (if (Utilities|IsValid _debug_widget)
      (Widget|RemovefromParent _debug_widget))))

(event EventBeginPlay
  (|CallParentFunction)
  (Variables|Default|SetMax%20Fingers%20Count 1))

(event EventTick
  (params (DeltaSeconds :type Float%20%28single-precision%29))
  (bind _target_delta (Variables|Temp|GetTarget%20Delta))
  (|CallParentFunction DeltaSeconds)
  (if (and (Variables|Configuration|GetEnable%20Interpolation) (Math|Vector|NotEqual(Vector) (Variables|Temp|GetCurrent%20Delta) _target_delta 0.01))
    (Default|CallOnDeltaXChanged (.X (Math|Vector|BreakVector (Math|Interpolation|VInterpTo (Variables|Temp|GetCurrent%20Delta) _target_delta DeltaSeconds (Variables|Configuration|GetInterpolation%20Speed)))))
    (Default|CallOnDeltaYChanged (.Y (Math|Vector|BreakVector (Math|Interpolation|VInterpTo (Variables|Temp|GetCurrent%20Delta) _target_delta DeltaSeconds (Variables|Configuration|GetInterpolation%20Speed)))))
    (Default|CallOnDeltaLocationChanged (Math|Interpolation|VInterpTo (Variables|Temp|GetCurrent%20Delta) _target_delta DeltaSeconds (Variables|Configuration|GetInterpolation%20Speed)))
    (Variables|Temp|SetCurrent%20Delta (Math|Interpolation|VInterpTo (Variables|Temp|GetCurrent%20Delta) _target_delta DeltaSeconds (Variables|Configuration|GetInterpolation%20Speed)))))

(event EventOnEventTouchPressed
  (params (Location :type Vector :default "0, 0, 0") (FingerIndex :type ETouchIndex%20Enum :default "Touch1"))
  (|CallParentFunction Location FingerIndex)
  (bind _output_get (Variables|Temp|SetPrevious%20Location Location))
  ;[0 0.25 1] Call Events
  (Default|CallOnPressed _output_get)
  ;[1 0.25 0] Debug Drawing with Special Debug Widget
  (if (Variables|Default|GetEnable%20Debug%20Drawing)
    (bind _returnvalue (UserInterface|CreateWidget "/Game/Blueprints/Touch/UTCDebugWidget.UTCDebugWidget_C"))
    (UserInterface|Viewport|AddtoViewport _returnvalue 0)
    (Variables|Temp|SetDebug%20Widget _returnvalue)
    (Variables|/Game/Blueprints/Touch/UTCDebugWidget.UTCDebugWidget_C|SetBounds%20Origin (Variables|Temp|GetDebug%20Widget) (Variables|Default|GetBounds%20Origin))
    (Variables|/Game/Blueprints/Touch/UTCDebugWidget.UTCDebugWidget_C|SetBound%20Size (Variables|Temp|GetDebug%20Widget) (Variables|Default|GetBounds%20Size))))

(fn RecalculateDelta
  (params (Current%20Location :type Vector))
  (bind _previous_location (Variables|Temp|GetPrevious%20Location))
  (bind _speed (Variables|Configuration|GetSpeed))
  (bind _returnvalue (- Current%20Location _previous_location))
  (bind _returnvalue_2 (/ 1.0 _speed))
  (bind _returnvalue_3 (/ _returnvalue _returnvalue_2))
  (return _returnvalue_3 (Math|Interpolation|VInterpTo (Variables|Temp|GetCurrent%20Delta) _returnvalue_3 (Utilities|Time|GetWorldDeltaSeconds) (Variables|Configuration|GetInterpolation%20Speed))))