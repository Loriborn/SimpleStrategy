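; Touch component that turns a two-finger gesture into pinch zoom, rotation and pan events.
; It builds on parent touch tracking, capturing length, angle and midpoint on second press, then broadcasting changes relative to them as fingers move.
; With ClampAfterRelease, Tick eases values back to their initial state after release, still firing move events.
; Optional debug tools draw the gesture in a widget and inject a stand-in second touch.
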(event EventBeginPlay
  (|CallParentFunction)
  (Variables|Default|SetMax%20Fingers%20Count 2))

(event EventTick
  (params (DeltaSeconds :type Float%20%28single-precision%29))
  (bind _initial_pan_location (Variables|Temp|GetInitial%20Pan%20Location))
  (bind _clamping_speed (Variables|Configuration|GetClamping%20Speed))
  (|CallParentFunction DeltaSeconds)
  (if (Math|Boolean|ANDBoolean (not (Variables|Temp|GetIs%20Two%20Fingers%20On%20Screen)) (Variables|Configuration|GetClamp%20After%20Release) (Math|Boolean|ORBoolean (!= (Variables|Temp|GetCurrent%20Length) (Variables|Temp|GetInitial%20Length)) (!= (Variables|Temp|GetCurrent%20Angle) (Variables|Temp|GetInitial%20Angle)) (Math|Vector|NotEqual(Vector) (Variables|Temp|GetCurrent%20Pan%20Location) (Variables|Temp|GetInitial%20Pan%20Location) 0.0)))
    (Variables|Temp|SetCurrent%20Angle (Math|Interpolation|FInterpTo (Variables|Temp|GetCurrent%20Angle) (Variables|Temp|GetInitial%20Angle) DeltaSeconds _clamping_speed))
    (Variables|Temp|SetCurrent%20Length (Math|Interpolation|FInterpTo (Variables|Temp|GetCurrent%20Length) (Variables|Temp|GetInitial%20Length) DeltaSeconds _clamping_speed))
    (Variables|Temp|SetCurrent%20Pan%20Location (Math|Interpolation|VInterpTo (Variables|Temp|GetCurrent%20Pan%20Location) (Variables|Temp|GetInitial%20Pan%20Location) DeltaSeconds _clamping_speed))
    ;[0 0.25 1] Call Events
    (Default|CallOnTwoFingersMove (/ (Variables|Temp|GetCurrent%20Length) (Variables|Temp|GetInitial%20Length)) (- (Variables|Temp|GetCurrent%20Angle) (Variables|Temp|GetInitial%20Angle)) _initial_pan_location (Variables|Temp|GetCurrent%20Pan%20Location) (- (Variables|Temp|GetCurrent%20Pan%20Location) _initial_pan_location))))

(event EventOnEventTouchPressed
  (params (Location :type Vector :default "0, 0, 0") (FingerIndex :type ETouchIndex%20Enum :default "Touch1"))
  (bind (_length _angle _halfway_vector) (CallFunction|GetLengthandAngle))
  (|CallParentFunction Location FingerIndex)
  (Utilities|FlowControl|Sequence
    (:then_0
      ;[1 0 0] Check and Set Fingers Count
      (CallFunction|CheckDebugTouchLocation) ; Check and restore debug touch location
      (if (== (CallFunction|GetFingersLength) (Variables|Default|GetMax%20Fingers%20Count))
        (if (not (Variables|Temp|GetIs%20Two%20Fingers%20On%20Screen))
          (Variables|Temp|SetIs%20Two%20Fingers%20On%20Screen true)
          ;[0 1 1] Setup
          (Variables|Temp|SetInitial%20Length _length)
          (Variables|Temp|SetInitial%20Angle _angle)
          (Variables|Temp|SetInitial%20Pan%20Location _halfway_vector)
          (Variables|Temp|SetCurrent%20Length _length)
          (Variables|Temp|SetCurrent%20Angle _angle)
          (bind _output_get (Variables|Temp|SetCurrent%20Pan%20Location _halfway_vector))
          ;[0 0.25 1] Call Events
          (Default|CallOnTwoFingersPressed _output_get)
          (Default|CallOnTwoFingersMove (/ (Variables|Temp|GetCurrent%20Length) (Variables|Temp|GetInitial%20Length)) (- (Variables|Temp|GetCurrent%20Angle) (Variables|Temp|GetInitial%20Angle)) (Variables|Temp|GetInitial%20Pan%20Location) (Variables|Temp|GetCurrent%20Pan%20Location) (- (Variables|Temp|GetCurrent%20Pan%20Location) (Variables|Temp|GetInitial%20Pan%20Location))))
        (else
          (Variables|Temp|SetIs%20Two%20Fingers%20On%20Screen false))))
    (:then_1
      ;[1 0.25 0] Draw Debug Widget
      (CallFunction|InitializeDebugWidget))))

(event EventOnEventTouchMoved
  (params (Location :type Vector :default "0, 0, 0") (FingerIndex :type ETouchIndex%20Enum :default "Touch1"))
  (bind (_length _angle _halfway_vector) (CallFunction|GetLengthandAngle))
  (bind _initial_pan_location (Variables|Temp|GetInitial%20Pan%20Location))
  (|CallParentFunction Location FingerIndex)
  (Utilities|FlowControl|Sequence
    (:then_0
      (if (Variables|Temp|GetIs%20Two%20Fingers%20On%20Screen)
        ;[0 1 1] Update
        (Variables|Temp|SetCurrent%20Length _length)
        (Variables|Temp|SetCurrent%20Angle _angle)
        (Variables|Temp|SetCurrent%20Pan%20Location _halfway_vector)
        ;[0 0.25 1] Call Events
        (Default|CallOnTwoFingersMove (/ (Variables|Temp|GetCurrent%20Length) (Variables|Temp|GetInitial%20Length)) (- (Variables|Temp|GetCurrent%20Angle) (Variables|Temp|GetInitial%20Angle)) _initial_pan_location (Variables|Temp|GetCurrent%20Pan%20Location) (- (Variables|Temp|GetCurrent%20Pan%20Location) _initial_pan_location))))
    (:then_1
      ;[1 0.25 0] Draw Debug Widget
      (CallFunction|UpdateDebugWidget))))

(event EventOnEventTouchReleased
  (params (Location :type Vector :default "0, 0, 0") (FingerIndex :type ETouchIndex%20Enum :default "Touch1"))
  (bind _current_pan_location (Variables|Temp|GetCurrent%20Pan%20Location))
  (bind _initial_pan_location (Variables|Temp|GetInitial%20Pan%20Location))
  (|CallParentFunction Location FingerIndex)
  (Utilities|FlowControl|Sequence
    (:then_0
      ;[0 1 1] Reset
      (Variables|Temp|SetIs%20Two%20Fingers%20On%20Screen false)
      ;[0 0.25 1] Call Events
      (if (== (CallFunction|GetFingersLength) 1)
        (Default|CallOnTwoFingersReleased (/ (Variables|Temp|GetCurrent%20Length) (Variables|Temp|GetInitial%20Length)) (- (Variables|Temp|GetCurrent%20Angle) (Variables|Temp|GetInitial%20Angle)) _initial_pan_location _current_pan_location (- _current_pan_location _initial_pan_location))))
    (:then_1
      ;[1 0.25 0] Draw Debug Widget
      (CallFunction|UninitializeDebugWidget))))

(fn UpdateDebugWidget
  (bind _debug_widget (Variables|Temp|GetDebug%20Widget))
  (if (and (Variables|Default|GetEnable%20Debug%20Drawing) (!= (Variables|Temp|GetDebug%20Widget) 0))
    (Variables|/Game/Blueprints/Touch/UTCPinchDebugWidget.UTCPinchDebugWidget_C|SetBounds%20Origin _debug_widget (Variables|Default|GetBounds%20Origin))
    (Variables|/Game/Blueprints/Touch/UTCPinchDebugWidget.UTCPinchDebugWidget_C|SetBound%20Size _debug_widget (Variables|Default|GetBounds%20Size))
    (Variables|/Game/Blueprints/Touch/UTCPinchDebugWidget.UTCPinchDebugWidget_C|SetFinger%20Locations _debug_widget (Variables|Default|GetLocations))
    (Variables|/Game/Blueprints/Touch/UTCPinchDebugWidget.UTCPinchDebugWidget_C|SetPan%20Location _debug_widget (Variables|Temp|GetCurrent%20Pan%20Location))))

(fn GetLengthandAngle
  (bind _locations (Variables|Default|GetLocations))
  (bind _output (Utilities|Array|Get(acopy) _locations))
  (bind _output_2 (Utilities|Array|Get(acopy) _locations 1))
  (bind _returnvalue (- _output _output_2))
  (bind _returnvalue_2 (Math|Vector|VectorLength _returnvalue))
  (bind _returnvalue_3 (Math|Vector|Normalize _returnvalue))
  (return _returnvalue_2 (Class|KismetMathLibrary|DegAtan2 (Math|Vector|DotProduct (Variables|Default|GetScreen%20Right%20Vector) _returnvalue_3) (Math|Vector|DotProduct (Variables|Default|GetScreen%20Up%20Vector) _returnvalue_3)) (- _output (* _returnvalue_3 (/ _returnvalue_2 2.0)))))

(fn InitializeDebugWidget
  (Utilities|FlowControl|Sequence
    (:then_0
      (if (and (Variables|Default|GetEnable%20Debug%20Drawing) (== (Variables|Temp|GetDebug%20Widget) 0))
        (bind _returnvalue (UserInterface|CreateWidget "/Game/Blueprints/Touch/UTCPinchDebugWidget.UTCPinchDebugWidget_C"))
        (UserInterface|Viewport|AddtoViewport _returnvalue 0)
        (Variables|Temp|SetDebug%20Widget _returnvalue)))
    (:then_1
      (CallFunction|UpdateDebugWidget))))

(fn UninitializeDebugWidget
  (if (and (Variables|Default|GetEnable%20Debug%20Drawing) (== (CallFunction|GetFingersLength) 0))
    (Widget|RemovefromParent (Variables|Temp|GetDebug%20Widget))
    (Variables|Temp|SetDebug%20Widget 0)
    (else
      (CallFunction|UpdateDebugWidget))))

(fn AddDebugTouchLocation
  (params (Location :type Vector))
  (bind _result (CallFunction|AddFingerLocation "Touch2" Location))
  (Variables|Temp|SetDebug%20Touch%20Location Location)
  (Variables|Temp|SetUse%20Debug%20Touch%20Location _result))

(fn RemoveDebugTouchLocation
  (CallFunction|RemoveFingerLocation "Touch2")
  (Variables|Temp|SetUse%20Debug%20Touch%20Location false))

(fn CheckDebugTouchLocation
  (if (and (Variables|Temp|GetUse%20Debug%20Touch%20Location) (not (CallFunction|IsFingerLocationExists "Touch2")))
    (CallFunction|AddDebugTouchLocation (Variables|Temp|GetDebug%20Touch%20Location))))