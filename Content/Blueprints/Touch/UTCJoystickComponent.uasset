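; Touch component that provides a single-finger virtual joystick with X/Y axis events, supporting fixed or floating placement, bounds and axis locking.
; Touch events update press and drag locations, from which magnitude, direction and angle feed per-tick axis values.
; On release, axes and picker interpolate back to rest before a clamped event fires.
; Custom widgets implementing IUTCWidget receive the events and can define the radius, with an optional debug overlay.
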(event Custom|On%20Joystick%20Location%20Changed%20Event
  (params (Location :type Vector))
  ;[0 1 1] Update Wigdet by Interface
  (Class|IUTCWidget|OnJoystickLocationChanged(Message) (Variables|UMGWidget|GetJoystick%20Widget) Location))

(event Custom|On%20Picker%20Location%20Changed%20Event
  (params (Location :type Vector))
  ;[0 1 1] Update Wigdet by Interface
  (Class|IUTCWidget|OnPickerLocationChanged(Message) (Variables|UMGWidget|GetJoystick%20Widget) Location))

(event Custom|On%20Viewport%20Size%20Changed%20Event
  (params (Previous%20Size :type Vector%202D%20Structure) (Updated%20Size :type Vector%202D%20Structure))
  ;[0 1 1] Update Wigdet by Interface
  (Class|IUTCWidget|OnViewportSizeChanged(Message) (Variables|UMGWidget|GetJoystick%20Widget) Previous%20Size Updated%20Size))

(event Custom|On%20Joystick%20Pressed%20Event
  (params (Location :type Vector))
  ;[0 1 1] Update Wigdet by Interface
  (Class|IUTCWidget|OnJoystickPressed(Message) (Variables|UMGWidget|GetJoystick%20Widget) Location))

(event Custom|On%20Joystick%20Released%20Event
  (params (Location :type Vector))
  ;[0 1 1] Update Wigdet by Interface
  (Class|IUTCWidget|OnJoystickReleased(Message) (Variables|UMGWidget|GetJoystick%20Widget) Location))

(event Custom|On%20Joystick%20Clamped%20Event
  ;[0 1 1] Update Wigdet by Interface
  (Class|IUTCWidget|OnJoystickClamped(Message) (Variables|UMGWidget|GetJoystick%20Widget)))

(event Custom|On%20X%20Axis%20Changed%20Event
  (params (Value :type Float%20%28single-precision%29))
  ;[0 1 1] Update Wigdet by Interface
  (Class|IUTCWidget|OnXAxisChanged(Message) (Variables|UMGWidget|GetJoystick%20Widget) Value))

(event Custom|On%20Y%20Axis%20Changed%20Event
  (params (Value :type Float%20%28single-precision%29))
  ;[0 1 1] Update Wigdet by Interface
  (Class|IUTCWidget|OnYAxisChanged(Message) (Variables|UMGWidget|GetJoystick%20Widget) Value))

(event Custom|On%20Axes%20Changed%20Event
  (params (XAxis :type Float%20%28single-precision%29) (YAxis :type Float%20%28single-precision%29) (Direction :type Vector))
  ;[0 1 1] Update Wigdet by Interface
  (Class|IUTCWidget|OnAxesChanged(Message) (Variables|UMGWidget|GetJoystick%20Widget) XAxis YAxis Direction))

(event Custom|Setup%20Widget
  (params (Widget%20%28with%20IUTCWIdget%20Interface%29 :type User%20Widget%20Class%20Reference) (Use%20Widget%20Size%20%28back%20texture%20size%29 :type Boolean) (Hide%20if%20pawn%20Unpossessed :type Boolean))
  ;[0 1 0] Setup Custom Widget
  (CallFunction|DestroyWidget)
  (bind _is_initialized (UMGWidget|InnerSetupWidget Widget%20%28with%20IUTCWIdget%20Interface%29 Use%20Widget%20Size%20%28back%20texture%20size%29 Hide%20if%20pawn%20Unpossessed))
  (if _is_initialized
    ;[0 1 1] Update Wigdet by Interface
    (EventDispatchers|BindEventtoOnJoystickLocationChanged (delegate Custom|On%20Joystick%20Location%20Changed%20Event))
    (EventDispatchers|BindEventtoOnPickerLocationChanged (delegate Custom|On%20Picker%20Location%20Changed%20Event))
    (EventDispatchers|BindEventtoOnJoystickPressed (delegate Custom|On%20Joystick%20Pressed%20Event))
    (EventDispatchers|BindEventtoOnJoystickReleased (delegate Custom|On%20Joystick%20Released%20Event))
    (EventDispatchers|BindEventtoOnJoystickClamped (delegate Custom|On%20Joystick%20Clamped%20Event))
    (EventDispatchers|BindEventtoOnXAxisChanged (delegate Custom|On%20X%20Axis%20Changed%20Event))
    (EventDispatchers|BindEventtoOnYAxisChanged (delegate Custom|On%20Y%20Axis%20Changed%20Event))
    (EventDispatchers|BindEventtoOnAxesChanged (delegate Custom|On%20Axes%20Changed%20Event))
    (EventDispatchers|AssignOnViewportSizeChanged (delegate Custom|On%20Viewport%20Size%20Changed%20Event))))

(event Custom|Destroy%20Widget
  (bind _joystick_widget (Variables|UMGWidget|GetJoystick%20Widget))
  ;[1 0.5 0] Destroy Custom Widget
  (if (Utilities|IsValid _joystick_widget)
    (Widget|RemovefromParent _joystick_widget)
    (EventDispatchers|UnbindEventfromOnJoystickLocationChanged (delegate Custom|On%20Joystick%20Location%20Changed%20Event))
    (EventDispatchers|UnbindEventfromOnPickerLocationChanged (delegate Custom|On%20Picker%20Location%20Changed%20Event))
    (EventDispatchers|UnbindEventfromOnJoystickPressed (delegate Custom|On%20Joystick%20Pressed%20Event))
    (EventDispatchers|UnbindEventfromOnJoystickReleased (delegate Custom|On%20Joystick%20Released%20Event))
    (EventDispatchers|UnbindEventfromOnJoystickClamped (delegate Custom|On%20Joystick%20Clamped%20Event))
    (EventDispatchers|UnbindEventfromOnXAxisChanged (delegate Custom|On%20X%20Axis%20Changed%20Event))
    (EventDispatchers|UnbindEventfromOnYAxisChanged (delegate Custom|On%20Y%20Axis%20Changed%20Event))
    (EventDispatchers|UnbindEventfromOnAxesChanged (delegate Custom|On%20Axes%20Changed%20Event))))

(event EventOnPawnPossesed
  (params (New%20Controller :type Controller%20Object%20Reference))
  (|CallParentFunction New%20Controller)
  ;[0 1 1] Show/hide joystick by pawn possesed/unpossesed events
  (Utilities|Casting|CastToPlayerController New%20Controller)
  (if (Utilities|IsValid (Variables|UMGWidget|GetJoystick%20Widget))
    (Widget|SetVisibility (Variables|UMGWidget|GetJoystick%20Widget) "Visible")
    (Bounds|SnapWidgettoBounds)))

(event EventOnViewportSizeIsChanged
  (UMGWidget|UpdateMagnitugebyWidgetSize)
  (FixedLocation|UpdateFixedLocation true)
  (CallFunction|SnapBoundstoFixedLocation)
  (Bounds|SnapWidgettoBounds))

(event EventOnEventTouchMoved
  (params (Location :type Vector :default "0, 0, 0") (FingerIndex :type ETouchIndex%20Enum :default "Touch1"))
  (bind _debug_widget (Variables|Temp|GetDebug%20Widget))
  (|CallParentFunction Location FingerIndex)
  (Utilities|IsJoystickPressedBranch FingerIndex
    (:True
      ;[0 1 1] Update
      (Variables|Temp|SetDrag%20Location Location)
      (CallFunction|UpdateTempVariables)
      (bind _joysticklocation (CallFunction|UpdateFloating))
      (CallFunction|UpdateLockAxes)
      ;[0 0.25 1] Call Events
      (Default|CallOnJoystickLocationChanged _joysticklocation)
      (Default|CallOnPickerLocationChanged (Variables|Temp|GetDrag%20Location))
      ;[1 0.25 0] Debug Drawing with Special Debug Widget
      (if (Variables|Default|GetEnable%20Debug%20Drawing)
        (Variables|/Game/Blueprints/Touch/UTCJoystickDebugWidget.UTCJoystickDebugWidget_C|SetJoystick%20Location _debug_widget (Math|Conversions|ToVector2D(Vector) (Variables|Temp|GetPress%20Location)))
        (Variables|/Game/Blueprints/Touch/UTCJoystickDebugWidget.UTCJoystickDebugWidget_C|SetPicker%20Location _debug_widget (Math|Conversions|ToVector2D(Vector) (Variables|Temp|GetDrag%20Location)))
        (Variables|/Game/Blueprints/Touch/UTCJoystickDebugWidget.UTCJoystickDebugWidget_C|SetBounds%20Origin _debug_widget (Variables|Default|GetBounds%20Origin))
        (Variables|/Game/Blueprints/Touch/UTCJoystickDebugWidget.UTCJoystickDebugWidget_C|SetBound%20Size (stale EventOnEventTouchPressed _output_get_3) (Variables|Default|GetBounds%20Size))))))

(event EventOnEventTouchReleased
  (params (Location :type Vector :default "0, 0, 0") (FingerIndex :type ETouchIndex%20Enum :default "Touch1"))
  (|CallParentFunction Location FingerIndex)
  (Utilities|IsJoystickPressedBranch FingerIndex
    (:True
      ;[0 1 1] Reset
      (Variables|Temp|SetReleased true)
      (Variables|Temp|SetMagnitude 0.0)
      (Variables|Temp|SetAngle 0.0)
      ;[0 0.25 1] Call Events
      (Default|CallOnJoystickReleased Location)
      ;[1 0.25 0] Debug Drawing with Special Debug Widget
      (if (Variables|Default|GetEnable%20Debug%20Drawing)
        (Widget|RemovefromParent (Variables|Temp|GetDebug%20Widget))))))

(event EventOnPawnUnpossesed
  (params (Old%20Controller :type Controller%20Object%20Reference))
  (|CallParentFunction Old%20Controller)
  ;[0 1 1] Show/hide joystick by pawn possesed/unpossesed events
  (if (Utilities|IsValid (Variables|UMGWidget|GetJoystick%20Widget))
    (if (Variables|UMGWidget|GetHide%20On%20Unpossession)
      (Widget|SetVisibility (Variables|UMGWidget|GetJoystick%20Widget) "Collapsed"))))

(event EventTick
  (params (DeltaSeconds :type Float%20%28single-precision%29))
  (bind _press_location (Variables|Temp|GetPress%20Location))
  (bind (_x _y) (Math|Vector|BreakVector _press_location))
  (|CallParentFunction DeltaSeconds)
  (if (Variables|Temp|GetReleased)
    (Utilities|FlowControl|Sequence
      (:then_0
        (if (or (!= (.X (Math|Vector2D|BreakVector2D (Variables|Temp|GetAxes))) 0.0) (!= (.Y (Math|Vector2D|BreakVector2D (Variables|Temp|GetAxes))) 0.0))
          (bind _output_get (Variables|Temp|SetAxes (Class|KismetMathLibrary|Vector2DInterpto (Variables|Temp|GetAxes) "(X=0.000000,Y=0.000000)" DeltaSeconds (Variables|Configuration|GetClamping%20Speed))))
          ;[0 0.25 1] Call Events
          (Default|CallOnXAxisChanged (.X (Math|Vector2D|BreakVector2D _output_get)))
          (Default|CallOnYAxisChanged (.Y (Math|Vector2D|BreakVector2D _output_get)))
          (Default|CallOnAxesChanged (.X (Math|Vector2D|BreakVector2D _output_get)) (.Y (Math|Vector2D|BreakVector2D _output_get)) (Variables|Temp|GetDirection))))
      (:then_1
        (if (or (!= _x (.X (Math|Vector|BreakVector (Variables|Temp|GetDrag%20Location)))) (!= _y (.Y (Math|Vector|BreakVector (Variables|Temp|GetDrag%20Location)))))
          (bind _output_get_2 (Variables|Temp|SetDrag%20Location (Math|Interpolation|VInterpTo (Variables|Temp|GetDrag%20Location) (Variables|Temp|GetPress%20Location) DeltaSeconds (Variables|Configuration|GetClamping%20Speed))))
          (Default|CallOnPickerLocationChanged _output_get_2)))
      (:then_2
        (if (not (and (or (!= (.X (Math|Vector2D|BreakVector2D (Variables|Temp|GetAxes))) 0.0) (!= (.Y (Math|Vector2D|BreakVector2D (Variables|Temp|GetAxes))) 0.0)) (or (!= _x (.X (Math|Vector|BreakVector (Variables|Temp|GetDrag%20Location)))) (!= _y (.Y (Math|Vector|BreakVector (Variables|Temp|GetDrag%20Location)))))))
          (Utilities|FlowControl|DoOnce true :!label _label
            (:Completed
              (Default|CallOnJoystickClamped))))))
    (else
      (Utilities|FlowControl|Sequence
        (:then_0
          (goto _label Reset))
        (:then_1
          (bind _axis (CallFunction|UpdateAxisVector))
          (Default|CallOnXAxisChanged (.X (Math|Vector2D|BreakVector2D _axis)))
          (Default|CallOnYAxisChanged (.Y (Math|Vector2D|BreakVector2D _axis)))
          (Default|CallOnAxesChanged (.X (Math|Vector2D|BreakVector2D _axis)) (.Y (Math|Vector2D|BreakVector2D _axis)) (Variables|Temp|GetDirection)))))))

(event EventBeginPlay
  (|CallParentFunction)
  (Variables|Default|SetMax%20Fingers%20Count 1))

(event EventOnEventTouchPressed
  (params (Location :type Vector :default "0, 0, 0") (FingerIndex :type ETouchIndex%20Enum :default "Touch1"))
  (|CallParentFunction Location FingerIndex)
  (Utilities|IsFingerLocationExistsBranch FingerIndex)
  ;[1 0 0] Prevent multiple entry by the same index (if PIE)
  (Utilities|IsJoystickPressedBranch FingerIndex
    (:True
      (CallFunction|OnEventTouchReleased Location FingerIndex))
    (:False
      _))
  (bind _location_out (Utilities|IsFixedLocationBranch Location))
  ;[0 1 1] Setup
  (Variables|Temp|SetCurrentFingerIndex FingerIndex)
  (bind _output_get (Variables|Temp|SetPress%20Location _location_out))
  (bind _output_get_2 (Variables|Temp|SetDrag%20Location Location))
  (Utilities|UpdateDragLocationinCaseOfFixedLocation
    (:True
      _)
    (:False
      _))
  (Variables|Temp|SetReleased false)
  ;[1 0 0.47] Immediate Recalculation with Fixed Location
  (if (and (Variables|FixedLocation|GetUse%20Fixed%20Location) (Variables|FixedLocation|GetRecalculate%20Immediately))
    (CallFunction|UpdateTempVariables))
  ;[0 0.25 1] Call Events
  (Default|CallOnJoystickPressed _output_get_2)
  (Default|CallOnJoystickLocationChanged _output_get)
  (Default|CallOnPickerLocationChanged _output_get_2)
  ;[1 0.25 0] Debug Drawing with Special Debug Widget
  (if (Variables|Default|GetEnable%20Debug%20Drawing)
    (bind _returnvalue (UserInterface|CreateWidget "/Game/Blueprints/Touch/UTCJoystickDebugWidget.UTCJoystickDebugWidget_C"))
    (UserInterface|Viewport|AddtoViewport _returnvalue 0)
    (bind _output_get_3 (Variables|Temp|SetDebug%20Widget _returnvalue))
    (Variables|/Game/Blueprints/Touch/UTCJoystickDebugWidget.UTCJoystickDebugWidget_C|SetJoystick%20Location _output_get_3 (Math|Conversions|ToVector2D(Vector) (Variables|Temp|GetPress%20Location)))
    (Variables|/Game/Blueprints/Touch/UTCJoystickDebugWidget.UTCJoystickDebugWidget_C|SetPicker%20Location _output_get_3 (Math|Conversions|ToVector2D(Vector) (Variables|Temp|GetDrag%20Location)))
    (Variables|/Game/Blueprints/Touch/UTCJoystickDebugWidget.UTCJoystickDebugWidget_C|SetRadius _output_get_3 (Variables|Configuration|GetMax%20Magnitude))
    (Variables|/Game/Blueprints/Touch/UTCJoystickDebugWidget.UTCJoystickDebugWidget_C|SetLockedAxis _output_get_3 (Variables|Configuration|GetLock%20Axis))
    (Variables|/Game/Blueprints/Touch/UTCJoystickDebugWidget.UTCJoystickDebugWidget_C|SetBounds%20Origin (Variables|Temp|GetDebug%20Widget) (Variables|Default|GetBounds%20Origin))
    (Variables|/Game/Blueprints/Touch/UTCJoystickDebugWidget.UTCJoystickDebugWidget_C|SetBound%20Size _output_get_3 (Variables|Default|GetBounds%20Size))))

(fn UpdateAxisVector
  (bind _magnitude (Variables|Temp|GetMagnitude))
  (bind _max_magnitude (Variables|Configuration|GetMax%20Magnitude))
  (bind _angle (Variables|Temp|GetAngle))
  (bind _joystick_offset (Variables|Configuration|GetJoystick%20Offset))
  (bind _direction (Variables|Temp|GetDirection))
  (bind _returnvalue (/ _magnitude _max_magnitude))
  (bind _returnvalue_2 (Math|Trig|Sin(Degrees) _angle))
  (bind _returnvalue_3 (Math|Trig|Cos(Degrees) _angle))
  (bind (_x _y) (Math|Vector|BreakVector _direction))
  (bind _returnvalue_4 (< _returnvalue 1.0))
  (bind _returnvalue_5 (Math|Float|SelectFloat _returnvalue 1.0 _returnvalue_4))
  (bind _returnvalue_6 (* _returnvalue_2 _returnvalue_5 _joystick_offset))
  (bind _returnvalue_7 (* _returnvalue_3 _returnvalue_5 _joystick_offset))
  (bind _returnvalue_8 (Math|Float|Absolute(Float) _returnvalue_6))
  (bind _returnvalue_9 (Math|Float|Absolute(Float) _returnvalue_7))
  (bind _output_get (Variables|Temp|SetAxes (Math|Vector2D|MakeVector2D (Math|Float|SelectFloat (* (Math|Float|SelectFloat 1.0 _returnvalue_8 (> _returnvalue_8 1.0)) (Math|Float|SelectFloat 1.0 -1.0 (> _x 0.0))) 0.0 (Utilities|Enum|NotEqual(Enum) (Variables|Configuration|GetLock%20Axis) "NewEnumerator1")) (Math|Float|SelectFloat (* (Math|Float|SelectFloat 1.0 _returnvalue_9 (> _returnvalue_9 1.0)) (Math|Float|SelectFloat -1.0 1.0 (> _y 0.0))) 0.0 (Utilities|Enum|NotEqual(Enum) (Variables|Configuration|GetLock%20Axis) "NewEnumerator2")))))
  (return _output_get))

(fn UpdateFloating
  (bind _magnitude (Variables|Temp|GetMagnitude))
  (bind _max_magnitude (Variables|Configuration|GetMax%20Magnitude))
  (bind _joystick_offset (Variables|Configuration|GetJoystick%20Offset))
  (bind _previous_magnitude (Variables|Temp|GetPrevious%20Magnitude))
  (bind _returnvalue (>= _previous_magnitude _magnitude))
  (bind _returnvalue_2 (!= _magnitude 0.0))
  (bind _returnvalue_3 (* _max_magnitude _joystick_offset))
  (bind _returnvalue_4 (<= _magnitude _returnvalue_3))
  (bind _returnvalue_5 (< _previous_magnitude _returnvalue_3))
  (bind _returnvalue_6 (Math|Float|SelectFloat _magnitude 0.01 _returnvalue_2))
  (bind _returnvalue_7 (- _magnitude _returnvalue_3))
  (bind _returnvalue_8 (/ _returnvalue_7 _returnvalue_6))
  (bind _returnvalue_9 (and _returnvalue _returnvalue_5))
  (bind _returnvalue_10 (or _returnvalue_9 _returnvalue_4))
  (if (and (Variables|Configuration|GetEnable%20Floating) (not (Variables|FixedLocation|GetUse%20Fixed%20Location)))
    (if (Variables|Default|GetUse%20Bounds)
      (bind (_in_bounds _w_out_bounds _in_bounds_by_x _in_bounds_by_y) (CallFunction|CheckBounds (Variables|Temp|GetDrag%20Location)))
      (Variables|Temp|SetPress%20Location (Math|Vector|SelectVector (Math|Vector|MakeVector (Math|Float|SelectFloat (.X (Math|Vector|BreakVector (Math|Vector|Lerp(Vector) (Variables|Temp|GetPress%20Location) (Variables|Temp|GetDrag%20Location) _returnvalue_8))) (.X (Math|Vector|BreakVector (Variables|Temp|GetPress%20Location))) _in_bounds_by_x) (Math|Float|SelectFloat (.Y (Math|Vector|BreakVector (Math|Vector|Lerp(Vector) (Variables|Temp|GetPress%20Location) (Variables|Temp|GetDrag%20Location) _returnvalue_8))) (.Y (Math|Vector|BreakVector (Variables|Temp|GetPress%20Location))) _in_bounds_by_y) 0.0) (Variables|Temp|GetPress%20Location) (not (and _returnvalue_10 _in_bounds))))
      (Variables|Temp|SetDrag%20Location (Math|Vector|SelectVector (Variables|Temp|GetDrag%20Location) (+ (Variables|Temp|GetPress%20Location) (* (Variables|Temp|GetDirection) (Variables|Configuration|GetMax%20Magnitude))) (and _in_bounds _returnvalue_10)))
      (else
        (Variables|Temp|SetPress%20Location (Math|Vector|SelectVector (Math|Vector|Lerp(Vector) (Variables|Temp|GetPress%20Location) (Variables|Temp|GetDrag%20Location) _returnvalue_8) (Variables|Temp|GetPress%20Location) (not _returnvalue_10)))
        (Variables|Temp|SetDrag%20Location (Math|Vector|SelectVector (Variables|Temp|GetDrag%20Location) (+ (Variables|Temp|GetPress%20Location) (* (Variables|Temp|GetDirection) (Variables|Configuration|GetMax%20Magnitude))) _returnvalue_10) :!label _label)))
    (else
      (goto _label)))
  (return (Variables|Temp|GetPress%20Location) (Variables|Temp|GetDrag%20Location)))

(fn UpdateLockAxes
  (bind _returnvalue (Utilities|Time|GetWorldDeltaSeconds))
  (bind _lock_axis (Variables|Configuration|GetLock%20Axis))
  (bind _drag_location (Variables|Temp|GetDrag%20Location))
  (bind (_x _y) (Math|Vector|BreakVector _drag_location))
  (Utilities|UpdateDragLocationinCaseOfFixedLocation
    (:True
      _)
    (:False
      (if (Variables|Default|GetIs%20In%20Bounds)
        (Variables|Temp|SetPress%20Location (Math|Vector|MakeVector (Math|Float|SelectFloat (.X (Math|Vector|BreakVector (Variables|Temp|GetPress%20Location))) (Math|Interpolation|FInterpTo _x (.X (Math|Vector|BreakVector (Variables|Temp|GetPress%20Location))) _returnvalue 12.0) (Utilities|Enum|NotEqual(Enum) _lock_axis "NewEnumerator1")) (Math|Float|SelectFloat (.Y (Math|Vector|BreakVector (Variables|Temp|GetPress%20Location))) (Math|Interpolation|FInterpTo _y (.Y (Math|Vector|BreakVector (Variables|Temp|GetPress%20Location))) _returnvalue 12.0) (Utilities|Enum|NotEqual(Enum) _lock_axis "NewEnumerator2")) (.Z (Math|Vector|BreakVector (Variables|Temp|GetPress%20Location))))))))
  (return))

(fn ClearVectorZ
  (params (In%20Vector :type Vector))
  (bind (_x _y) (Math|Vector|BreakVector In%20Vector))
  (return (Math|Vector|MakeVector _x _y 0.0)))

(fn SnapWidgettoBounds
  (bind _joystick_widget (Variables|UMGWidget|GetJoystick%20Widget))
  (bind _fixed_location (Variables|FixedLocation|GetFixed%20Location))
  (bind _bounds_origin (Variables|Default|GetBounds%20Origin))
  (bind _bounds_size (Variables|Default|GetBounds%20Size))
  (bind _returnvalue (/ _bounds_size 2.0))
  (bind _returnvalue_2 (Math|Conversions|ToVector(Vector2D) _fixed_location))
  (bind _returnvalue_3 (+ _bounds_origin _returnvalue))
  (bind _returnvalue_4 (Math|Conversions|ToVector(Vector2D) _returnvalue_3))
  (if (Variables|FixedLocation|GetUse%20Fixed%20Location)
    (Class|IUTCWidget|OnJoystickLocationChanged(Message) _joystick_widget _returnvalue_2)
    (Class|IUTCWidget|OnPickerLocationChanged(Message) _joystick_widget _returnvalue_2)
    (elif (Variables|Default|GetUse%20Bounds)
      (Class|IUTCWidget|OnJoystickLocationChanged(Message) _joystick_widget _returnvalue_4)
      (Class|IUTCWidget|OnPickerLocationChanged(Message) _joystick_widget _returnvalue_4)))
  (return))

(fn GetJoystickWidgetInstance
  (return (Variables|UMGWidget|GetJoystick%20Widget)))

(fn InnerSetupWidget
  (params (Widget%20Class :type User%20Widget%20Class%20Reference) (Use%20Widget%20Size :type Boolean) (Hide%20If%20Unpossessed :type Boolean))
  (bind (_is_possessed_by_pc _is_locally_controlled) (CallFunction|GetIsPawnPossessedbyPC))
  (if (!= Widget%20Class "/Game/Blueprints/Touch/UTCJoystickDebugWidget.UTCJoystickDebugWidget_C")
    (Variables|UMGWidget|SetUse%20Widget%20Size Use%20Widget%20Size)
    (Variables|UMGWidget|SetHide%20On%20Unpossession Hide%20If%20Unpossessed)
    (bind _returnvalue (UserInterface|CreateWidget Widget%20Class))
    (if (Utilities|IsValid _returnvalue)
      (Utilities|Casting|CastToIUTCWidget _returnvalue
        (:then
          (UserInterface|Viewport|AddtoViewport _returnvalue 0)
          (Variables|UMGWidget|SetJoystick%20Widget _returnvalue)
          (if (Variables|UMGWidget|GetUse%20Widget%20Size)
            (bind _value (Class|IUTCWidget|GetMaxSize(Message) (Variables|UMGWidget|GetJoystick%20Widget)))
            (if (> _value 0.0)
              (Variables|Configuration|SetMax%20Magnitude (/ (* _value (Class|WidgetLayoutLibrary|GetViewportScale)) 2.0))
              (else
                (Development|PrintString "Error! Texture size cannot be zero. Please check your widget and override \"Get Background Texture Max Size\" function." true true "(R=1.000000,G=0.000000,B=0.000000,A=1.000000)" 3.0)
                (CallFunction|DestroyWidget)
                (return false)))
            (else
              (Class|IUTCWidget|SetMaxSize(Message) (Variables|UMGWidget|GetJoystick%20Widget) (* (/ (Variables|Configuration|GetMax%20Magnitude) (Class|WidgetLayoutLibrary|GetViewportScale)) 2.0))))
          (Bounds|SnapWidgettoBounds)
          (if (or (Math|Boolean|ANDBoolean (Variables|Default|GetOwner%20is%20Pawn%20or%20Controller) (Variables|UMGWidget|GetHide%20On%20Unpossession) (not _is_possessed_by_pc)) (not _is_locally_controlled))
            (Widget|SetVisibility (Variables|UMGWidget|GetJoystick%20Widget) "Collapsed"))
          (return true))
        (:CastFailed
          (Development|PrintString "Error! You're trying to create widget without IUTCWidget Interface.")))
      (else
        (Development|PrintString "Warning! You're trying to setup empty widget." false true "(R=1.000000,G=0.000000,B=0.000000,A=1.000000)" 3.0)))
    (else
      (Development|PrintString "Error! You can't use JoystickDebugWidget as custom UMG widget. To enable debug drawing use \"Enable Debug Drawing\" property." true true "(R=1.000000,G=0.000000,B=0.000000,A=1.000000)" 5.0)))
  (return false))

(fn GetDirectionAngle
  (return (Variables|Temp|GetAngle)))

(fn UpdateMagnitugebyWidgetSize
  (bind _joystick_widget (Variables|UMGWidget|GetJoystick%20Widget))
  (if (and (!= _joystick_widget 0) (Variables|UMGWidget|GetUse%20Widget%20Size))
    (bind _value (Class|IUTCWidget|GetMaxSize(Message) _joystick_widget))
    (if (> _value 0.0)
      (Variables|Configuration|SetMax%20Magnitude (/ (* _value (Class|WidgetLayoutLibrary|GetViewportScale)) 2.0)))))

(fn SetupFixedLocation
  (params (Is%20Enabled :type Boolean) (Fixed%20Location :type Vector%202D%20Structure) (In%20Percent :type Boolean) (Imeediate%20Recalculation :type Boolean) (Adjust%20Bounds%20to%20Fixed%20Location :type Boolean))
  (bind _output_get (Variables|FixedLocation|SetUse%20Fixed%20Location Is%20Enabled))
  (Variables|FixedLocation|SetRecalculate%20Immediately Imeediate%20Recalculation)
  (Variables|FixedLocation|SetAdjust%20Bounds%20to%20Fixed%20Location Adjust%20Bounds%20to%20Fixed%20Location)
  (if _output_get
    (if In%20Percent
      (Variables|FixedLocation|SetFixed%20Location%20%28%25%29 Fixed%20Location)
      (Variables|FixedLocation|SetUse%20Fixed%20Location%20In%20Percentage In%20Percent)
      (FixedLocation|UpdateFixedLocation true)
      (else
        (Variables|FixedLocation|SetFixed%20Location Fixed%20Location)))
    (CallFunction|SnapBoundstoFixedLocation)))

(fn UpdateFixedLocation
  (params (Is%20Viewport%20Size%20Changed :type Boolean))
  (bind _fixed_location____ (Variables|FixedLocation|GetFixed%20Location%20%28%25%29))
  (bind (_x _y) (Math|Vector2D|BreakVector2D _fixed_location____))
  (if (Math|Boolean|ANDBoolean Is%20Viewport%20Size%20Changed (Variables|FixedLocation|GetUse%20Fixed%20Location) (Variables|FixedLocation|GetUse%20Fixed%20Location%20In%20Percentage))
    (Variables|FixedLocation|SetFixed%20Location (Math|Vector2D|MakeVector2D (* _x (Math|Conversions|ToFloat(Integer) (Variables|Default|GetActual%20Viewport%20Size%20X))) (* _y (Math|Conversions|ToFloat(Integer) (Variables|Default|GetActual%20Viewport%20Size%20Y)))))))

(fn UpdateTempVariables
  (bind _drag_location (Variables|Temp|GetDrag%20Location))
  (bind _press_location (Variables|Temp|GetPress%20Location))
  (bind _returnvalue (- _drag_location _press_location))
  ;[0 1 1] Update required variables
  (Variables|Temp|SetPrevious%20Magnitude (Variables|Temp|GetMagnitude))
  (Variables|Temp|SetMagnitude (Math|Vector|VectorLength _returnvalue))
  (bind _output_get (Variables|Temp|SetDirection (Math|Vector|Normalize _returnvalue)))
  (Variables|Temp|SetAngle (Class|KismetMathLibrary|DegAcos (Math|Vector|DotProduct (Variables|Default|GetScreen%20Up%20Vector) _output_get))))

(fn SnapBoundstoFixedLocation
  (bind _max_magnitude (Variables|Configuration|GetMax%20Magnitude))
  (bind _returnvalue (Math|Vector2D|MakeVector2D _max_magnitude _max_magnitude))
  (if (and (Variables|FixedLocation|GetUse%20Fixed%20Location) (Variables|FixedLocation|GetAdjust%20Bounds%20to%20Fixed%20Location))
    (CallFunction|SetupBounds true (- (Variables|FixedLocation|GetFixed%20Location) _returnvalue) (* _returnvalue 2.0) false false)))