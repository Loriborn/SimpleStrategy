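; Touch control actor component for a Pawn or PlayerController that tracks fingers and their locations, with an empty resize hook suggesting a base class.
; Optional screen bounds, priority and active-state filters support choosing among components, while possession changes release touches and toggle a background widget.
; Tick watches viewport size to rescale percentage bounds and reposition that widget.
; It also polls until a controller loads, broadcasts connection, then disables polling on all Pawns' components.
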(event EventTick
  (params (DeltaSeconds :type Float%20%28single-precision%29))
  (Utilities|FlowControl|Sequence
    (:then_0
      (|ViewportChangingChecking))
    (:then_1
      (|NetworkConnectionChecking))))

(event EventBeginPlay
  (CallFunction|CheckIsViewportSizeChanged)
  (CallFunction|IsPawnPossessedbyPC))

(fn OnPawnPossesed
  (params (New%20Controller :type Controller%20Object%20Reference))
  (Variables|Temp|SetIs%20Possessed (Class|Controller|IsPlayerController New%20Controller))
  (Utilities|Casting|CastToPlayerController New%20Controller)
  (if (Utilities|IsValid (Variables|BackgroundWidget|GetBackground%20Widget))
    (Widget|SetVisibility (Variables|BackgroundWidget|GetBackground%20Widget) "Visible")))

(fn OnPawnUnpossesed
  (params (Old%20Controller :type Controller%20Object%20Reference))
  (Utilities|FlowControl|Sequence
    (:then_0
      (Utilities|Casting|CastToPlayerController Old%20Controller)
      (for (_array_element _array_index) (Variables|FingersLocations|GetFingers)
        (TouchEvents|OnEventTouchReleased (Utilities|Array|Get(acopy) (Variables|FingersLocations|GetLocations) _array_index) _array_element)
        (Variables|Temp|SetIs%20Possessed false)))
    (:then_1
      (if (Utilities|IsValid (Variables|BackgroundWidget|GetBackground%20Widget))
        (if (Variables|BackgroundWidget|GetBGW%20Hide%20if%20Pawn%20Unpossessed)
          (Widget|SetVisibility (Variables|BackgroundWidget|GetBackground%20Widget) "Collapsed"))))))

(fn OnEventTouchPressed
  (params (Location :type Vector) (FingerIndex :type ETouchIndex%20Enum :default "Touch1"))
  (FingersLocations|AddFingerLocation FingerIndex Location))

(fn OnEventTouchMoved
  (params (Location :type Vector) (FingerIndex :type ETouchIndex%20Enum :default "Touch1"))
  (FingersLocations|UpdateFingerLocation FingerIndex Location))

(fn OnEventTouchReleased
  (params (Location :type Vector) (FingerIndex :type ETouchIndex%20Enum :default "Touch1"))
  (FingersLocations|RemoveFingerLocation FingerIndex))

(fn CheckBounds
  (params (Location :type Vector))
  (bind (_x _y) (Math|Vector|BreakVector Location))
  (bind _bounds_origin (Variables|Bounds|GetBounds%20Origin))
  (bind _bounds_size (Variables|Bounds|GetBounds%20Size))
  (bind (_x_2 _y_2) (Math|Vector2D|BreakVector2D _bounds_origin))
  (bind (_x_3 _y_3) (Math|Vector2D|BreakVector2D _bounds_size))
  (bind _returnvalue (> _x _x_2))
  (bind _returnvalue_2 (> _y _y_2))
  (bind _returnvalue_3 (+ _x_2 _x_3))
  (bind _returnvalue_4 (+ _y_2 _y_3))
  (bind _returnvalue_5 (< _x _returnvalue_3))
  (bind _returnvalue_6 (< _y _returnvalue_4))
  (bind _returnvalue_7 (and _returnvalue _returnvalue_5))
  (bind _returnvalue_8 (and _returnvalue_2 _returnvalue_6))
  (if (Bounds|IsBoundingEnabled)
    (Variables|Temp|SetIs%20In%20Bounds (and _returnvalue_7 _returnvalue_8))
    (else
      (bind _output_get (Variables|Temp|SetIs%20In%20Bounds true))
      (LocalVariables|SetWithout%20Bounds _output_get)))
  (return (Variables|Temp|GetIs%20In%20Bounds) (LocalVariables|GetWithout%20Bounds) _returnvalue_7 _returnvalue_8))

(fn IsBoundingEnabled
  (bind _bounds_size (Variables|Bounds|GetBounds%20Size))
  (bind (_x _y) (Math|Vector2D|BreakVector2D _bounds_size))
  (return (not (or (not (Variables|Bounds|GetUse%20Bounds)) (and (== _x 0.0) (== _y 0.0))))))

(fn UpdateBoundsinPercent
  (params (Is%20Viewport%20Size%20Changed :type Boolean))
  (bind _bounds_origin____ (Variables|Bounds|GetBounds%20Origin%20%28%25%29))
  (bind _bounds_size____ (Variables|Bounds|GetBounds%20Size%20%28%25%29))
  (bind _actual_viewport_size_x (Variables|Temp|GetActual%20Viewport%20Size%20X))
  (bind _actual_viewport_size_y (Variables|Temp|GetActual%20Viewport%20Size%20Y))
  (bind _returnvalue (Math|Conversions|ToFloat(Integer) _actual_viewport_size_x))
  (bind _returnvalue_2 (Math|Conversions|ToFloat(Integer) _actual_viewport_size_y))
  (bind (_x _y) (Math|Vector2D|BreakVector2D _bounds_size____))
  (bind (_x_2 _y_2) (Math|Vector2D|BreakVector2D _bounds_origin____))
  (bind _returnvalue_3 (* _x _returnvalue))
  (bind _returnvalue_4 (* _y _returnvalue_2))
  (bind _returnvalue_5 (Math|Vector2D|MakeVector2D _returnvalue_3 _returnvalue_4))
  (bind (_x_3 _y_3) (Math|Vector2D|BreakVector2D _returnvalue_5))
  (bind _returnvalue_6 (Math|Float|Max(Float) _x_3 _y_3))
  (if (Math|Boolean|ANDBoolean Is%20Viewport%20Size%20Changed (Variables|Bounds|GetUse%20Bounds) (Variables|Bounds|GetBounds%20In%20Percentage))
    (Variables|Bounds|SetBounds%20Size (select (Variables|Bounds|GetRectangular%20%28by%20greater%20value%29) (Math|Vector2D|MakeVector2D _returnvalue_6 _returnvalue_6) _returnvalue_5))
    (Variables|Bounds|SetBounds%20Origin (Math|Vector2D|MakeVector2D (* _returnvalue _x_2) (* _returnvalue_2 _y_2)))))

(fn CheckIsViewportSizeChanged
  (bind _returnvalue (Viewport|GetViewportSize))
  (bind _returnvalue_2 (Math|Float|Truncate (.x _returnvalue)))
  (bind _returnvalue_3 (Math|Float|Truncate (.y _returnvalue)))
  (if (or (!= _returnvalue_2 (Variables|Temp|GetActual%20Viewport%20Size%20X)) (!= _returnvalue_3 (Variables|Temp|GetActual%20Viewport%20Size%20Y)))
    (Variables|Temp|SetActual%20Viewport%20Size%20X _returnvalue_2)
    (Variables|Temp|SetActual%20Viewport%20Size%20Y _returnvalue_3)
    (LocalVariables|SetIs%20Changed true))
  (return (LocalVariables|GetIs%20Changed)))

(fn AddFingerLocation
  (params (Finger%20Index :type ETouchIndex%20Enum :default "Touch1") (Location :type Vector))
  (Utilities|FlowControl|Sequence
    (:then_0
      (bind _returnvalue (Utilities|Array|Add (Variables|FingersLocations|GetFingers) Finger%20Index)))
    (:then_1
      (bind _returnvalue_2 (Utilities|Array|Add (Variables|FingersLocations|GetLocations) Location)))
    (:then_2
      (if (== _returnvalue _returnvalue_2)
        (return (== _returnvalue _returnvalue_2))
        (else
          (Utilities|FlowControl|Sequence
            (:then_0
              (Utilities|Array|RemoveIndex (Variables|FingersLocations|GetFingers) _returnvalue))
            (:then_1
              (Utilities|Array|RemoveIndex (Variables|FingersLocations|GetLocations) _returnvalue_2))
            (:then_2
              (return (== _returnvalue _returnvalue_2)))))))))

(fn RemoveFingerLocation
  (params (Finger%20Index :type ETouchIndex%20Enum :default "Touch1"))
  (bind _fingers (Variables|FingersLocations|GetFingers))
  (bind _returnvalue (Utilities|Array|FindItem _fingers Finger%20Index))
  (Utilities|Array|RemoveIndex (Variables|FingersLocations|GetLocations) _returnvalue)
  (Utilities|Array|RemoveIndex _fingers _returnvalue))

(fn UpdateFingerLocation
  (params (Finger%20Index :type ETouchIndex%20Enum :default "Touch1") (New%20Location :type Vector))
  (Utilities|Array|SetArrayElem (Variables|FingersLocations|GetLocations) (Utilities|Array|FindItem (Variables|FingersLocations|GetFingers) Finger%20Index) New%20Location))

(fn GetFingersLength
  (return (Utilities|Array|Length (Variables|FingersLocations|GetFingers))))

(fn IsFingerLocationExists
  (params (Finger%20Index :type ETouchIndex%20Enum :default "Touch1"))
  (return (Utilities|Array|IsValidIndex (Variables|FingersLocations|GetLocations) (Utilities|Array|FindItem (Variables|FingersLocations|GetFingers) Finger%20Index))))

(fn SortbyPriority
  (params (UTC%20Components :type Array%20of%20UTC%20Component%20Object%20References))
  (bind _w__higher_priority_local (LocalVariables|GetW/%20Higher%20Priority%20Local))
  (for _array_element UTC%20Components
    (if (> (Variables|UTCComponent_C|GetPriority _array_element) (LocalVariables|GetHigher%20Priority))
      (LocalVariables|SetHigher%20Priority (Variables|UTCComponent_C|GetPriority _array_element))))
  (for _array_element_2 UTC%20Components
    (if (== (Variables|UTCComponent_C|GetPriority _array_element_2) (LocalVariables|GetHigher%20Priority))
      (Utilities|Array|Add _w__higher_priority_local _array_element_2)))
  (return _w__higher_priority_local))

(fn FilterbyBounds
  (params (UTC%20Components :type Array%20of%20UTC%20Component%20Object%20References) (Location :type Vector))
  (bind _in_bounds_local (LocalVariables|GetIn%20Bounds%20Local))
  (bind _w_out_bounds_local (LocalVariables|GetW/out%20Bounds%20Local))
  (bind _both_local (LocalVariables|GetBoth%20Local))
  (for _array_element UTC%20Components
    (bind (_in_bounds _w_out_bounds) (Bounds|CheckBounds _array_element Location))
    (if (and _in_bounds (not _w_out_bounds))
      (Utilities|Array|Add _in_bounds_local _array_element)
      (Utilities|Array|Add _both_local _array_element :!label _label)
      (elif _w_out_bounds
        (Utilities|Array|Add _w_out_bounds_local _array_element)
        (goto _label))))
  (return _in_bounds_local _w_out_bounds_local _both_local))

(fn SetupBounds
  (params (Is%20Enabled :type Boolean) (Bounds%20Origin :type Vector%202D%20Structure) (Bounds%20Size :type Vector%202D%20Structure) (In%20Percent :type Boolean) (Rect%20%28by%20greater%20value%29 :type Boolean))
  (bind _output_get (Variables|Bounds|SetUse%20Bounds Is%20Enabled))
  (if _output_get
    (if In%20Percent
      (Variables|Bounds|SetBounds%20Origin%20%28%25%29 Bounds%20Origin)
      (Variables|Bounds|SetBounds%20Size%20%28%25%29 Bounds%20Size)
      (Variables|Bounds|SetRectangular%20%28by%20greater%20value%29 Rect%20%28by%20greater%20value%29)
      (Variables|Bounds|SetBounds%20In%20Percentage true)
      (Bounds|UpdateBoundsinPercent true)
      (else
        (Variables|Bounds|SetBounds%20Origin Bounds%20Origin)
        (Variables|Bounds|SetBounds%20Size Bounds%20Size)))))

(fn IsFingerSlotsAvailable
  (bind _max_fingers_count (Variables|Configuration|GetMax%20Fingers%20Count))
  (return (or (== _max_fingers_count 0) (> _max_fingers_count (FingersLocations|GetFingersLength)))))

(fn OnViewportSizeIsChanged)

(fn GetFingerIndexandLocationbyIndex
  (params (Index :type Integer))
  (bind _locations (Variables|FingersLocations|GetLocations))
  (bind _fingers (Variables|FingersLocations|GetFingers))
  (return (Utilities|Array|Get(acopy) _locations Index) (Utilities|Array|Get(acopy) _fingers Index) (and (Utilities|Array|IsValidIndex _locations Index) (Utilities|Array|IsValidIndex _fingers Index))))

(fn FilterbyActive
  (params (UTCComponents :type Array%20of%20UTC%20Component%20Object%20References))
  (bind _active_utc_components (LocalVariables|GetActive%20UTC%20Components))
  (for _array_element UTCComponents
    (if (Components|Activation|IsActive _array_element)
      (Utilities|Array|Add _active_utc_components _array_element)))
  (return _active_utc_components))

(fn GetIsPawnPossessedbyPC
  (bind _returnvalue (Components|GetOwner))
  (bind _aspawn (Utilities|Casting|CastToPawn _returnvalue)
    (:then
      (Variables|Temp|SetOwner%20is%20Pawn%20or%20Controller true)
      (Utilities|Casting|CastToPlayerController (Pawn|GetController _aspawn)
        (:then
          (bind _output_get (Variables|Temp|SetIs%20Possessed true)))
        (:CastFailed
          (Variables|Temp|SetIs%20Possessed false)))
      (return _output_get (Pawn|IsLocallyControlled _aspawn)))
    (:CastFailed
      (bind _asplayer_controller (Utilities|Casting|CastToPlayerController _returnvalue)
        (:then
          (Variables|Temp|SetOwner%20is%20Pawn%20or%20Controller true)
          (bind _output_get_2 (Variables|Temp|SetIs%20Possessed (Utilities|IsValid (Pawn|GetControlledPawn _asplayer_controller)))))
        (:CastFailed
          _))
      (return _output_get_2 (Pawn|IsLocalController _asplayer_controller)))))

(fn IsPawnPossessedbyPC
  (bind (_is_possessed_by_pc _is_locally_controlled) (CallFunction|GetIsPawnPossessedbyPC))
  (return _is_possessed_by_pc _is_locally_controlled))

(fn IsPlayerControllerLoaded
  (bind _returnvalue (Components|GetOwner))
  (bind _aspawn (Utilities|Casting|CastToPawn _returnvalue)
    (:then
      (return (Utilities|IsValid (Pawn|GetController _aspawn))))
    (:CastFailed
      (bind _ascontroller (Utilities|Casting|CastToController _returnvalue)
        (:then
          _)
        (:CastFailed
          _))
      (return (Utilities|IsValid _ascontroller)))))

(fn UpdateBackgroundWidget
  (bind _returnvalue (Class|WidgetLayoutLibrary|GetViewportScale))
  (bind _bgw_force_origin (Variables|BackgroundWidget|GetBGW%20Force%20Origin))
  (bind _background_widget (Variables|BackgroundWidget|GetBackground%20Widget))
  (bind _bgw_force_size (Variables|BackgroundWidget|GetBGW%20Force%20Size))
  (bind _bgw_size_in_percent (Variables|BackgroundWidget|GetBGW%20Size%20In%20Percent))
  (bind _bgw_use_bounds_size_and_origin (Variables|BackgroundWidget|GetBGW%20Use%20Bounds%20Size%20and%20Origin))
  (bind _returnvalue_2 (Utils|GetScreenSizebySizeinPercents _bgw_force_size))
  (bind _returnvalue_3 (select _bgw_size_in_percent _returnvalue_2 _bgw_force_size))
  (bind (_x _y) (Math|Vector2D|BreakVector2D _returnvalue_3))
  (bind _returnvalue_4 (Math|Float|Max(Float) _x _y))
  (if (Utilities|IsValid _background_widget)
    (Class|UserWidget|SetPositioninViewport _background_widget (select _bgw_use_bounds_size_and_origin (Variables|Bounds|GetBounds%20Origin) (select (Variables|BackgroundWidget|GetBGW%20Origin%20In%20Percent) (Utils|GetScreenSizebySizeinPercents _bgw_force_origin) _bgw_force_origin)) true)
    (Class|UserWidget|SetDesiredSizeinViewport _background_widget (/ (select _bgw_use_bounds_size_and_origin (Variables|Bounds|GetBounds%20Size) (select (Variables|BackgroundWidget|GetBGW%20Rectangular%20Size) (Math|Vector2D|MakeVector2D _returnvalue_4 _returnvalue_4) _returnvalue_3)) (Math|Float|SelectFloat _returnvalue 1.0 (!= _returnvalue 0.0))))))

(fn SetupBackgroundWidget
  (params (Background%20Widget%20Class :type User%20Widget%20Class%20Reference) (Hide%20if%20Pawn%20Unpossessed :type Boolean) (Use%20Bounds%20Size%20and%20Origin :type Boolean) (Origin%20%28if%20you're%20not%20using%20bounds%29 :type Vector%202D%20Structure) (Origin%20In%20Percent :type Boolean) (Size%20%28if%20you're%20not%20using%20bounds%29 :type Vector%202D%20Structure) (Size%20In%20Percent :type Boolean) (Rectangular%20%28by%20greater%20value%20of%20Size%29 :type Boolean))
  (bind (_is_possessed_by_pc _is_locally_controlled) (CallFunction|GetIsPawnPossessedbyPC))
  (if (Utilities|IsValidClass Background%20Widget%20Class)
    (Utilities|FlowControl|Sequence
      (:then_0
        ;[0 0.2823 1] Set/Update variables
        (Variables|BackgroundWidget|SetBGW%20Hide%20if%20Pawn%20Unpossessed Hide%20if%20Pawn%20Unpossessed)
        (Variables|BackgroundWidget|SetBGW%20Use%20Bounds%20Size%20and%20Origin Use%20Bounds%20Size%20and%20Origin)
        (Variables|BackgroundWidget|SetBGW%20Force%20Size Size%20%28if%20you're%20not%20using%20bounds%29)
        (Variables|BackgroundWidget|SetBGW%20Force%20Origin Origin%20%28if%20you're%20not%20using%20bounds%29)
        (Variables|BackgroundWidget|SetBGW%20Origin%20In%20Percent Origin%20In%20Percent)
        (Variables|BackgroundWidget|SetBGW%20Rectangular%20Size Rectangular%20%28by%20greater%20value%20of%20Size%29)
        (Variables|BackgroundWidget|SetBGW%20Size%20In%20Percent Size%20In%20Percent)
        (if (Utilities|IsValid (Variables|BackgroundWidget|GetBackground%20Widget))
          ;[1 0.00692 0] Removing existing bg widget if class is different
          (if (!= (Utilities|GetClass (Variables|BackgroundWidget|GetBackground%20Widget)) Background%20Widget%20Class)
            (Widget|RemovefromParent (Variables|BackgroundWidget|GetBackground%20Widget))
            ;[0.007439 1 0] Creating new bg widget
            (bind _returnvalue (UserInterface|CreateWidget Background%20Widget%20Class :!label _label))
            (UserInterface|Viewport|AddtoViewport _returnvalue 0)
            (bind _output_get (Variables|BackgroundWidget|SetBackground%20Widget _returnvalue))
            (if (or (Math|Boolean|ANDBoolean (Variables|Temp|GetOwner%20is%20Pawn%20or%20Controller) (Variables|BackgroundWidget|GetBGW%20Hide%20if%20Pawn%20Unpossessed) (not _is_possessed_by_pc)) (not _is_locally_controlled))
              (Widget|SetVisibility _output_get "Collapsed")))
          (else
            (goto _label))))
      (:then_1
        (BackgroundWidget|UpdateBackgroundWidget)))
    (else
      ;[1 0.006541 0] Removing existing bg widget if class is null
      (if (Utilities|IsValid (Variables|BackgroundWidget|GetBackground%20Widget))
        (Widget|RemovefromParent (Variables|BackgroundWidget|GetBackground%20Widget))))))

(fn GetScreenSizebySizeinPercents
  (params (InVec :type Vector%202D%20Structure))
  (bind (_x _y) (Math|Vector2D|BreakVector2D InVec))
  (return (Math|Vector2D|MakeVector2D (* _x (Math|Conversions|ToFloat(Integer) (Variables|Temp|GetActual%20Viewport%20Size%20X))) (* _y (Math|Conversions|ToFloat(Integer) (Variables|Temp|GetActual%20Viewport%20Size%20Y))))))

(fn SetupBackgroundbyBounds
  (params (Background%20Widget%20Class :type User%20Widget%20Class%20Reference) (Hide%20if%20Pawn%20Unpossessed :type Boolean))
  (BackgroundWidget|SetupBackgroundWidget :Background%20Widget%20Class Background%20Widget%20Class :Hide%20if%20Pawn%20Unpossessed Hide%20if%20Pawn%20Unpossessed))

(fn SetupBackgroundbySizeandOrigin
  (params (Widget%20Class :type User%20Widget%20Class%20Reference) (Hide%20if%20Pawn%20Unpossessed :type Boolean) (Origin :type Vector%202D%20Structure) (Origin%20In%20Percent :type Boolean) (Size :type Vector%202D%20Structure) (Size%20In%20Percent :type Boolean) (Rectangular%20%28by%20greater%20value%20of%20Size%29 :type Boolean))
  (BackgroundWidget|SetupBackgroundWidget Widget%20Class Hide%20if%20Pawn%20Unpossessed false Origin Origin%20In%20Percent Size Size%20In%20Percent Rectangular%20%28by%20greater%20value%20of%20Size%29))

(event Custom|Disable%20Network%20Connection%20Checking
  ;[0 1 0] Disable network checking for all other pawn (other clients)
  (Variables|Configuration|SetCheck%20Network%20Connection false))