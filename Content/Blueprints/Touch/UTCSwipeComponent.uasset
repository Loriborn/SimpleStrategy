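; Single-finger touch component that detects a swipe at a required angle and reports success or failure with locations, timing and an eight-way direction.
; A swipe must exceed a fraction of the shorter viewport side and fall within a wrapped angle tolerance measured against screen up.
; It evaluates on release, or during movement once long enough if ImmediateCall is set, then drops the finger.
; An optional debug widget visualises the gesture and its thresholds.
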(event EventBeginPlay
  (|CallParentFunction)
  (Variables|Default|SetMax%20Fingers%20Count 1))

(event EventTick
  (params (DeltaSeconds :type Float%20%28single-precision%29))
  (|CallParentFunction DeltaSeconds))

(event EventOnEventTouchPressed
  (params (Location :type Vector :default "0, 0, 0") (FingerIndex :type ETouchIndex%20Enum :default "Touch1"))
  (|CallParentFunction Location FingerIndex)
  ;[1 0.25 0] Draw Debug Widget
  (Utilities|FlowControl|Sequence
    (:then_0
      ;[0 1 1] Setup
      (bind _output_get (Variables|Temp|SetPress%20Location Location))
      (Variables|Temp|SetDrag/Release%20Location _output_get)
      (Variables|Temp|SetPress%20Time (Math|DateTime|Now)))
    (:then_1
      (CallFunction|InitializeDebugWidget))))

(event EventOnEventTouchMoved
  (params (Location :type Vector :default "0, 0, 0") (FingerIndex :type ETouchIndex%20Enum :default "Touch1"))
  (bind _returnvalue (Math|DateTime|Now))
  (bind _press_time (Variables|Temp|GetPress%20Time))
  (bind _press_location (Variables|Temp|GetPress%20Location))
  (bind _returnvalue_2 (- _returnvalue _press_time))
  (|CallParentFunction Location FingerIndex)
  ;[1 0.25 0] Draw Debug Widget
  (Utilities|FlowControl|Sequence
    (:then_0
      ;[0 1 1] Update
      (Variables|Temp|SetDrag/Release%20Location Location)
      (if (Variables|Configuration|GetImmediate%20Call)
        (bind _output_get (Variables|Temp|SetDirection (Math|Vector|Normalize (- (Variables|Temp|GetDrag/Release%20Location) (Variables|Temp|GetPress%20Location)))))
        ;[1 0 0] Check
        (if (CallFunction|IsLengthMatch (Math|Vector|VectorLength (- (Variables|Temp|GetDrag/Release%20Location) (Variables|Temp|GetPress%20Location))))
          (CallFunction|RemoveFingerLocation FingerIndex)
          (if (CallFunction|IsAngleMatch (Class|KismetMathLibrary|DegAtan2 (Math|Vector|DotProduct (Variables|Default|GetScreen%20Right%20Vector) _output_get) (Math|Vector|DotProduct (Variables|Default|GetScreen%20Up%20Vector) _output_get)))
            ;[0 0.25 1] Call Events
            (Default|CallOnSwipeGestureSuccess _press_location (Variables|Temp|GetDrag/Release%20Location) (Variables|Temp|GetDirection) _returnvalue_2 (CallFunction|GetSwipeDirection (Class|KismetMathLibrary|DegAtan2 (Math|Vector|DotProduct (Variables|Default|GetScreen%20Right%20Vector) _output_get) (Math|Vector|DotProduct (Variables|Default|GetScreen%20Up%20Vector) _output_get))))
            (else
              (Default|CallOnSwipeGestureFail _press_location (Variables|Temp|GetDrag/Release%20Location) (Variables|Temp|GetDirection) _returnvalue_2 (CallFunction|GetSwipeDirection (Class|KismetMathLibrary|DegAtan2 (Math|Vector|DotProduct (Variables|Default|GetScreen%20Right%20Vector) _output_get) (Math|Vector|DotProduct (Variables|Default|GetScreen%20Up%20Vector) _output_get))))))
          ;[1 0.25 0] Remove Debug Widget
          (CallFunction|UninitializeDebugWidget))))
    (:then_1
      (CallFunction|UpdateDebugWidget))))

(event EventOnEventTouchReleased
  (params (Location :type Vector :default "0, 0, 0") (FingerIndex :type ETouchIndex%20Enum :default "Touch1"))
  (bind _returnvalue (Math|DateTime|Now))
  (bind _press_time (Variables|Temp|GetPress%20Time))
  (bind _press_location (Variables|Temp|GetPress%20Location))
  (bind _returnvalue_2 (- _returnvalue _press_time))
  (|CallParentFunction Location FingerIndex)
  ;[0 1 1] Update
  (Variables|Temp|SetDrag/Release%20Location Location)
  (Variables|Temp|SetDirection (Math|Vector|Normalize (- (Variables|Temp|GetDrag/Release%20Location) (Variables|Temp|GetPress%20Location))))
  ;[1 0 0] Check
  (if (CallFunction|IsLengthMatch (Math|Vector|VectorLength (- (Variables|Temp|GetDrag/Release%20Location) (Variables|Temp|GetPress%20Location))))
    (if (CallFunction|IsAngleMatch (Class|KismetMathLibrary|DegAtan2 (Math|Vector|DotProduct (Variables|Default|GetScreen%20Right%20Vector) (stale EventOnEventTouchMoved _output_get)) (Math|Vector|DotProduct (Variables|Default|GetScreen%20Up%20Vector) (stale EventOnEventTouchMoved _output_get))))
      ;[0 0.25 1] Call Events
      (Default|CallOnSwipeGestureSuccess _press_location (Variables|Temp|GetDrag/Release%20Location) (Variables|Temp|GetDirection) _returnvalue_2 (CallFunction|GetSwipeDirection (Class|KismetMathLibrary|DegAtan2 (Math|Vector|DotProduct (Variables|Default|GetScreen%20Right%20Vector) (stale EventOnEventTouchMoved _output_get)) (Math|Vector|DotProduct (Variables|Default|GetScreen%20Up%20Vector) (stale EventOnEventTouchMoved _output_get)))))
      (else
        (Default|CallOnSwipeGestureFail _press_location (Variables|Temp|GetDrag/Release%20Location) (Variables|Temp|GetDirection) _returnvalue_2 (CallFunction|GetSwipeDirection (Class|KismetMathLibrary|DegAtan2 (Math|Vector|DotProduct (Variables|Default|GetScreen%20Right%20Vector) (stale EventOnEventTouchMoved _output_get)) (Math|Vector|DotProduct (Variables|Default|GetScreen%20Up%20Vector) (stale EventOnEventTouchMoved _output_get)))) :!label _label)))
    (else
      (goto _label)))
  ;[1 0.25 0] Remove Debug Widget
  (CallFunction|UninitializeDebugWidget))

(fn IsLengthMatch
  (params (Length :type Float%20%28single-precision%29))
  (return (> Length (* (Math|Integer|Min(Integer) (Variables|Default|GetActual%20Viewport%20Size%20X) (Variables|Default|GetActual%20Viewport%20Size%20Y)) (Variables|Configuration|GetRequired%20Length%20%28in%20%25%20of%20lower%20side%29)))))

(fn GetSwipeDirection
  (params (Angle :type Float%20%28single-precision%29))
  (return (Utilities|Enum|ByteToEnumEUTCSwipeDirection (Math|Conversions|ToByte(Integer) (Math|Integer|SelectInt 0 (Math|Integer|SelectInt 1 (Math|Integer|SelectInt 2 (Math|Integer|SelectInt 3 (Math|Integer|SelectInt 4 (Math|Integer|SelectInt 5 (Math|Integer|SelectInt 6 (Math|Integer|SelectInt 7 0 (and (>= Angle -67.5) (< Angle -22.5))) (and (>= Angle -112.5) (< Angle -67.5))) (and (>= Angle -157.5) (< Angle -112.5))) (or (and (>= Angle 157.5) (<= Angle 1.8e+02)) (and (>= Angle -1.8e+02) (< Angle -157.5)))) (and (>= Angle 112.5) (< Angle 157.5))) (and (>= Angle 67.5) (< Angle 112.5))) (and (>= Angle 22.5) (< Angle 67.5))) (and (>= Angle -22.5) (< Angle 22.5)))))))

(fn InitializeDebugWidget
  (Utilities|FlowControl|Sequence
    (:then_0
      (if (Variables|Default|GetEnable%20Debug%20Drawing)
        (bind _returnvalue (UserInterface|CreateWidget "/Game/Blueprints/Touch/UTCSwipeDebugWidget.UTCSwipeDebugWidget_C"))
        (UserInterface|Viewport|AddtoViewport _returnvalue 0)
        (Variables|Temp|SetDebug%20Widget _returnvalue)))
    (:then_1
      (CallFunction|UpdateDebugWidget))))

(fn UpdateDebugWidget
  (bind _debug_widget (Variables|Temp|GetDebug%20Widget))
  (if (Variables|Default|GetEnable%20Debug%20Drawing)
    (Variables|/Game/Blueprints/Touch/UTCSwipeDebugWidget.UTCSwipeDebugWidget_C|SetPress%20Location _debug_widget (Math|Conversions|ToVector2D(Vector) (Variables|Temp|GetPress%20Location)))
    (Variables|/Game/Blueprints/Touch/UTCSwipeDebugWidget.UTCSwipeDebugWidget_C|SetDrag%20Location _debug_widget (Math|Conversions|ToVector2D(Vector) (Variables|Temp|GetDrag/Release%20Location)))
    (Variables|/Game/Blueprints/Touch/UTCSwipeDebugWidget.UTCSwipeDebugWidget_C|SetBounds%20Origin _debug_widget (Variables|Default|GetBounds%20Origin))
    (Variables|/Game/Blueprints/Touch/UTCSwipeDebugWidget.UTCSwipeDebugWidget_C|SetBound%20Size _debug_widget (Variables|Default|GetBounds%20Size))
    (Variables|/Game/Blueprints/Touch/UTCSwipeDebugWidget.UTCSwipeDebugWidget_C|SetRequired%20Length _debug_widget (* (Math|Integer|Min(Integer) (Variables|Default|GetActual%20Viewport%20Size%20X) (Variables|Default|GetActual%20Viewport%20Size%20Y)) (Variables|Configuration|GetRequired%20Length%20%28in%20%25%20of%20lower%20side%29)))
    (Variables|/Game/Blueprints/Touch/UTCSwipeDebugWidget.UTCSwipeDebugWidget_C|SetRequired%20Angle _debug_widget (Variables|Configuration|GetRequired%20Angle))
    (Variables|/Game/Blueprints/Touch/UTCSwipeDebugWidget.UTCSwipeDebugWidget_C|SetError%20Tolerance _debug_widget (Variables|Configuration|GetAngle%20Error%20Tolerance%20%28in%20degrees%29))))

(fn UninitializeDebugWidget
  (if (Variables|Default|GetEnable%20Debug%20Drawing)
    (Widget|RemovefromParent (Variables|Temp|GetDebug%20Widget))))

(fn IsAngleMatch
  (params (Angle :type Float%20%28single-precision%29))
  (bind _required_angle (Variables|Configuration|GetRequired%20Angle))
  (bind _returnvalue (- Angle _required_angle))
  (return (<= (Math|Float|Absolute(Float) (- _returnvalue (* 3.6e+02 (Math|Conversions|ToFloat(Integer) (Math|Float|Floor (/ (+ _returnvalue 1.8e+02) 3.6e+02)))))) (Variables|Configuration|GetAngle%20Error%20Tolerance%20%28in%20degrees%29))))