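; Touch gesture component that detects one- and two-finger taps and double taps, and raises events for them plus move and release.
; Each press compares stored timestamps against interval thresholds, resetting to epoch after a double tap; late second fingers raise a failure event.
; Taps fire immediately on press, so a double tap follows a single-tap event.
; Optional debug drawing shows tap locations and bounds in a viewport widget, removed on release.
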(event EventTick
  (params (DeltaSeconds :type Float%20%28single-precision%29))
  (|CallParentFunction DeltaSeconds))

(event EventOnEventTouchReleased
  (params (Location :type Vector :default "0, 0, 0") (FingerIndex :type ETouchIndex%20Enum :default "Touch1"))
  (|CallParentFunction Location FingerIndex)
  ;[0 0.25 1] Call Events (one finger tap)
  (Default|CallOnTapRelease Location FingerIndex)
  ;[1 0.25 0] Debug Drawing with Special Debug Widget
  (if (Variables|Default|GetEnable%20Debug%20Drawing)
    (Widget|RemovefromParent (Variables|Temp|GetDebug%20Widget))
    (Variables|Temp|SetDebug%20Widget 0)))

(event EventBeginPlay
  (|CallParentFunction)
  (Variables|Default|SetMax%20Fingers%20Count 2))

(event EventOnEventTouchPressed
  (params (Location :type Vector :default "0, 0, 0") (FingerIndex :type ETouchIndex%20Enum :default "Touch1"))
  (bind (_location _fingerindex) (CallFunction|GetFingerIndexandLocationbyIndex 1))
  (bind (_location_2 _fingerindex_2) (CallFunction|GetFingerIndexandLocationbyIndex))
  (bind _debug_widget (Variables|Temp|GetDebug%20Widget))
  (bind _debug_widget_2 (Variables|Temp|GetDebug%20Widget))
  (|CallParentFunction Location FingerIndex)
  ;[1 0 0] Check for fingers count (is two?)
  (if (== (CallFunction|GetFingersLength) (Variables|Default|GetMax%20Fingers%20Count))
    ;[1 0 0] Check for two fingers tap
    (if (< (Class|KismetMathLibrary|GetTotalMilliseconds (- (Math|DateTime|Now) (Variables|Temp|GetLast%20Tap%20Time))) (Variables|Configuration|GetTwo%20Fingers%20Tap%20Interval%20%28ms%29))
      ;[1 0 0] Check for two fingers double tap
      (if (< (Class|KismetMathLibrary|GetTotalMilliseconds (- (Math|DateTime|Now) (Variables|Temp|GetTwo%20Fingers%20Tap%20Time))) (Variables|Configuration|GetDouble%20Tap%20Interval%20%28ms%29))
        ;[0 1 1] Setup (two fingers tap)
        (Variables|Temp|SetTwo%20Fingers%20Tap%20Time (Math|DateTime|MakeDateTime 1970 1 1))
        ;[0 0.25 1] Call Events (two fingers tap)
        (Default|CallOnTwoFingersDoubleTap _location_2 _fingerindex_2 _location _fingerindex (Class|KismetMathLibrary|GetTotalMilliseconds (- (Math|DateTime|Now) (Variables|Temp|GetTwo%20Fingers%20Tap%20Time))))
        ;[1 0.25 0] Debug Drawing with Special Debug Widget
        (Utilities|InitializeDebugWidgetMacro
          (:On%20Initialized
            (Variables|/Game/Blueprints/Touch/UTCTapDebugWidget.UTCTapDebugWidget_C|SetDouble%20Tap _debug_widget true)))
        (else
          (Variables|Temp|SetTwo%20Fingers%20Tap%20Time (Math|DateTime|Now))
          (Default|CallOnTwoFingersTap _location_2 _fingerindex_2 _location _fingerindex)
          (Utilities|InitializeDebugWidgetMacro
            (:On%20Initialized
              _))))
      (Variables|/Game/Blueprints/Touch/UTCTapDebugWidget.UTCTapDebugWidget_C|SetTap%20Locations _debug_widget (Utilities|Array|MakeArray (Math|Conversions|ToVector2D(Vector) _location_2) (Math|Conversions|ToVector2D(Vector) _location)))
      (Variables|/Game/Blueprints/Touch/UTCDebugWidget.UTCDebugWidget_C|SetBound%20Size _debug_widget_2 (Variables|Default|GetBounds%20Size) :!label _label)
      (Variables|/Game/Blueprints/Touch/UTCDebugWidget.UTCDebugWidget_C|SetBounds%20Origin _debug_widget_2 (Variables|Default|GetBounds%20Origin))
      (else
        (Default|CallOnTwoFingersTapFailed "Time interval between two touches is too big." (Class|KismetMathLibrary|GetTotalMilliseconds (- (Math|DateTime|Now) (Variables|Temp|GetLast%20Tap%20Time))))))
    (else
      (Variables|Temp|SetLast%20Tap%20Time (Math|DateTime|Now))
      ;[1 0 0] Double Tap Check
      (if (< (Class|KismetMathLibrary|GetTotalMilliseconds (- (Variables|Temp|GetLast%20Tap%20Time) (Variables|Temp|GetOne%20Finger%20Tap%20Time))) (Variables|Configuration|GetDouble%20Tap%20Interval%20%28ms%29))
        ;[0 1 1] Setup (one finger tap)
        (Variables|Temp|SetOne%20Finger%20Tap%20Time (Math|DateTime|MakeDateTime 1970 1 1))
        ;[0 0.25 1] Call Events (one finger tap)
        (Default|CallOnDoubleTap Location FingerIndex (Class|KismetMathLibrary|GetTotalMilliseconds (- (Variables|Temp|GetLast%20Tap%20Time) (Variables|Temp|GetOne%20Finger%20Tap%20Time))))
        (Utilities|InitializeDebugWidgetMacro
          (:On%20Initialized
            (Variables|/Game/Blueprints/Touch/UTCTapDebugWidget.UTCTapDebugWidget_C|SetDouble%20Tap _debug_widget_2 true)))
        (else
          (Variables|Temp|SetOne%20Finger%20Tap%20Time (Variables|Temp|GetLast%20Tap%20Time))
          (Default|CallOnTap Location FingerIndex)
          (Utilities|InitializeDebugWidgetMacro
            (:On%20Initialized
              _))))
      (Variables|/Game/Blueprints/Touch/UTCTapDebugWidget.UTCTapDebugWidget_C|SetTap%20Locations _debug_widget_2 (Utilities|Array|MakeArray (Math|Conversions|ToVector2D(Vector) Location)))
      (goto _label))))

(event EventOnEventTouchMoved
  (params (Location :type Vector :default "0, 0, 0") (FingerIndex :type ETouchIndex%20Enum :default "Touch1"))
  (bind _debug_widget (Variables|Temp|GetDebug%20Widget))
  (|CallParentFunction Location FingerIndex)
  ;[0 0.25 1] Call Events (one finger tap)
  (Default|CallOnTapMove Location FingerIndex)
  ;[1 0.25 0] Debug Drawing with Special Debug Widget
  (if (Variables|Default|GetEnable%20Debug%20Drawing)
    (Variables|/Game/Blueprints/Touch/UTCDebugWidget.UTCDebugWidget_C|SetBound%20Size _debug_widget (Variables|Default|GetBounds%20Size))
    (Variables|/Game/Blueprints/Touch/UTCDebugWidget.UTCDebugWidget_C|SetBounds%20Origin _debug_widget (Variables|Default|GetBounds%20Origin))))

(fn InitializeDebugWidget
  (if (Variables|Default|GetEnable%20Debug%20Drawing)
    (if (Utilities|IsValid (Variables|Temp|GetDebug%20Widget))
      _
      (else
        (bind _returnvalue (UserInterface|CreateWidget "/Game/Blueprints/Touch/UTCTapDebugWidget.UTCTapDebugWidget_C"))
        (UserInterface|Viewport|AddtoViewport _returnvalue 0)
        (Variables|Temp|SetDebug%20Widget _returnvalue)))
    (Variables|/Game/Blueprints/Touch/UTCTapDebugWidget.UTCTapDebugWidget_C|SetBounds%20Origin (Variables|Temp|GetDebug%20Widget) (Variables|Default|GetBounds%20Origin))
    (Variables|/Game/Blueprints/Touch/UTCTapDebugWidget.UTCTapDebugWidget_C|SetBound%20Size (Variables|Temp|GetDebug%20Widget) (Variables|Default|GetBounds%20Size))
    (Variables|/Game/Blueprints/Touch/UTCTapDebugWidget.UTCTapDebugWidget_C|SetDouble%20Tap (Variables|Temp|GetDebug%20Widget) false)
    (return true)
    (else
      (return false))))